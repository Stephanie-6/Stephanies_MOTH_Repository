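; Key pickup actor that gives the player a key when interacted with.
; On Interact it plays a pickup sound, adds its KeyId to the FirstPersonCharacter and posts a timed feed message with the key name.
; Flags control whether it also adds a journal entry and whether it destroys itself afterward.
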(event `/Game/Blueprints/Interaction_interface.Interact`
  (bind _asfirst_person_character (cast `/Game/FirstPersonBP/Blueprints/FirstPersonCharacter` (`GameplayStatics.GetPlayerCharacter` 0)))
  (`GameplayStatics.PlaySoundAtLocation` "/Game/HorrorEngine/Audio/Environment/TakeKey.TakeKey" (`self.K2_GetActorLocation`) (struct) 1.0 1.0 0.0 null null null)
  (`/Game/FirstPersonBP/Blueprints/FirstPersonCharacter.AddKey` _asfirst_person_character (`self.key_id`))
  (bind _asfirst_person_character_2 (cast `/Game/FirstPersonBP/Blueprints/FirstPersonCharacter` (`GameplayStatics.GetPlayerCharacter` 0)))
  (`/Game/FirstPersonBP/Blueprints/FirstPersonCharacter.AddFeedEntry` _asfirst_person_character_2 (make `/Game/Blueprints/FeedItem` (`KismetTextLibrary.Conv_StringToText` (`KismetStringLibrary.Concat_StrStr` (`self.key_name`) " obtained"))))
  (if (`self.add_journal_entry`)
    (`/Game/FirstPersonBP/Blueprints/FirstPersonCharacter.AddJournalEntry` _asfirst_person_character_2 (`self.journal entry`)))
  (if (`self.destroyOnPickup`)
    (`self.K2_DestroyActor`)))

(fn `UserConstructionScript`)