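; An interactable painting Blueprint that hands the player a key the first time it is used.
; Interact clears the Active flag, plays a creak sound, and gives the FirstPersonCharacter the key Id, a timed feed message and a journal entry.
; It then zeroes the actor's relative roll, keeping pitch and yaw, so a tilted painting straightens.
; The construction script applies the configurable painting material to the mesh.
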(event `/Game/Blueprints/Interaction_interface.Interact`
  (bind (_relativerotation_roll _relativerotation_pitch _relativerotation_yaw) (`KismetMathLibrary.BreakRotator` (`SceneComponent.RelativeRotation` (`self.DefaultSceneRoot`))))
  (if (`self.active`)
    (set `self.active` false)
    (bind _asfirst_person_character (cast `/Game/FirstPersonBP/Blueprints/FirstPersonCharacter` (`GameplayStatics.GetPlayerCharacter` 0)))
    (`GameplayStatics.PlaySoundAtLocation` "/Game/HorrorEngine/Audio/DoorsAndFurnitures/Creak10.Creak10" (`self.K2_GetActorLocation`) (struct) 1.0 1.0 0.0 null null null)
    (`/Game/FirstPersonBP/Blueprints/FirstPersonCharacter.AddKey` _asfirst_person_character (`self.id`))
    (bind _asfirst_person_character_2 (cast `/Game/FirstPersonBP/Blueprints/FirstPersonCharacter` (`GameplayStatics.GetPlayerCharacter` 0)))
    (`/Game/FirstPersonBP/Blueprints/FirstPersonCharacter.AddFeedEntry` _asfirst_person_character_2 (make `/Game/Blueprints/FeedItem` (`KismetTextLibrary.Conv_StringToText` (`KismetStringLibrary.Concat_StrStr` (`self.Key_Named`) " obtained"))))
    (`/Game/FirstPersonBP/Blueprints/FirstPersonCharacter.AddJournalEntry` _asfirst_person_character_2 (`self.journal_entry`))
    (`self.K2_SetActorRelativeRotation` (`KismetMathLibrary.MakeRotator` 0.0 _relativerotation_pitch _relativerotation_yaw))))

(fn `UserConstructionScript`
  (`PrimitiveComponent.SetMaterial` (`self.painting`) 0 (`self.painting _mat`)))